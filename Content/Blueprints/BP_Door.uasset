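; BP_Door is a broken door the player repairs with components, then opens and closes with E.
; Front and back triggers enable input and show prompts; holding E runs a timer that activates the door, consumes components and plays a sound.
; Tick lights repaired doors and ramps leakage lights while bleeding blue and closed.
; A phasing event briefly shifts collision, then clears bleeding; overlaps flag contact with BP_BlueGhost.
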(event OnComponentBeginOverlap(DoorCollision)
  (params (OverlappedComponent :type Primitive%20Component%20Object%20Reference) (OtherActor :type Actor%20Object%20Reference) (OtherComp :type Primitive%20Component%20Object%20Reference) (OtherBodyIndex :type Integer) (bFromSweep :type Boolean) (SweepResult :type Hit%20Result%20Structure%20%28by%20ref%29))
  (Utilities|Casting|CastToBP_BlueGhost OtherActor)
  (Variables|Default|SetIsDoorTouchingGhost true))

(event OnComponentEndOverlap(BackCollision)
  (params (OverlappedComponent :type Primitive%20Component%20Object%20Reference) (OtherActor :type Actor%20Object%20Reference) (OtherComp :type Primitive%20Component%20Object%20Reference) (OtherBodyIndex :type Integer))
  (Utilities|Casting|CastToBP_FirstPersonCharacter OtherActor)
  (Input|DisableInput (Game|GetPlayerController 0))
  (Rendering|Components|TextRender|SetText (Variables|Default|GetBackText) (Utilities|Text|ToText(String) "")))

(event OnComponentEndOverlap(DoorCollision)
  (params (OverlappedComponent :type Primitive%20Component%20Object%20Reference) (OtherActor :type Actor%20Object%20Reference) (OtherComp :type Primitive%20Component%20Object%20Reference) (OtherBodyIndex :type Integer))
  (Utilities|Casting|CastToBP_BlueGhost OtherActor)
  (Variables|Default|SetIsDoorTouchingGhost false))

(event OnComponentBeginOverlap(FrontCollision)
  (params (OverlappedComponent :type Primitive%20Component%20Object%20Reference) (OtherActor :type Actor%20Object%20Reference) (OtherComp :type Primitive%20Component%20Object%20Reference) (OtherBodyIndex :type Integer) (bFromSweep :type Boolean) (SweepResult :type Hit%20Result%20Structure%20%28by%20ref%29))
  (bind _asbp_first_person_character (Utilities|Casting|CastToBP_FirstPersonCharacter OtherActor))
  (Utilities|FlowControl|Sequence
    (:then_0
      (Input|EnableInput (Game|GetPlayerController 0))
      (if (not (Variables|Default|GetIsActive))
        (Rendering|Components|TextRender|SetText (Variables|Default|GetFrontText) (Utilities|Text|ToText(String) "Hold E to Fix the Door"))))
    (:then_1
      (Variables|Default|SetCharacterReference _asbp_first_person_character))))

(event OnComponentEndOverlap(FrontCollision)
  (params (OverlappedComponent :type Primitive%20Component%20Object%20Reference) (OtherActor :type Actor%20Object%20Reference) (OtherComp :type Primitive%20Component%20Object%20Reference) (OtherBodyIndex :type Integer))
  (Utilities|Casting|CastToBP_FirstPersonCharacter OtherActor)
  (Input|DisableInput (Game|GetPlayerController 0))
  (Rendering|Components|TextRender|SetText (Variables|Default|GetFrontText) (Utilities|Text|ToText(String) "")))

(event OnComponentBeginOverlap(BackCollision)
  (params (OverlappedComponent :type Primitive%20Component%20Object%20Reference) (OtherActor :type Actor%20Object%20Reference) (OtherComp :type Primitive%20Component%20Object%20Reference) (OtherBodyIndex :type Integer) (bFromSweep :type Boolean) (SweepResult :type Hit%20Result%20Structure%20%28by%20ref%29))
  (bind _asbp_first_person_character (Utilities|Casting|CastToBP_FirstPersonCharacter OtherActor))
  (Utilities|FlowControl|Sequence
    (:then_0
      (Input|EnableInput (Game|GetPlayerController 0))
      (if (not (Variables|Default|GetIsActive))
        (Rendering|Components|TextRender|SetText (Variables|Default|GetBackText) (Utilities|Text|ToText(String) "Press E to Fix the Door"))))
    (:then_1
      (Variables|Default|SetCharacterReference _asbp_first_person_character))))

(event Custom|FixDoor
  (Variables|Default|SetIsActive true)
  (Rendering|Components|TextRender|SetText (Variables|Default|GetFrontText) (Utilities|Text|ToText(String) "Press E to Open and Close"))
  (Default|ConsumeComponents (Variables|Default|GetCharacterReference))
  (Audio|Components|Audio|Play (Variables|Default|GetSound) 0.0))

(event Custom|MakeDoorTemporarilyPhasable
  (Transformation|AddLocalOffset (Variables|Default|GetDoorCollision) "0.000000,0.000000,330.000000" false false)
  (Utilities|Time|SetTimerbyEvent (delegate Custom|RecloseDoor) 0.4))

(event Custom|RecloseDoor
  (Transformation|AddLocalOffset (Variables|Default|GetDoorCollision) "0.000000,0.000000,-330.000000" false false)
  (Variables|Default|SetIsBleedingBlue false))

(event EventTick
  (params (DeltaSeconds :type Float%20%28single-precision%29))
  (Utilities|FlowControl|Sequence
    (:then_0
      (if (Variables|Default|GetIsActive)
        (Rendering|Material|SetMaterial (Variables|Default|GetDoorLight) 0 "/Game/Materials/M_Light.M_Light")))
    (:then_1
      (if (Variables|Default|GetIsBleedingBlue)
        (if (not (Variables|Default|GetIsOpen))
          (bind _output_get (Variables|Default|SetIntensity (Variables|/Script/Engine.LightComponentBase|GetIntensity (Variables|Default|GetLeakage1))))
          (Rendering|Components|Light|SetIntensity (Variables|Default|GetLeakage2) (+ _output_get 0.05)))
        (else
          (Rendering|Components|Light|SetIntensity (Variables|Default|GetLeakage2) 0.0))))))

(event Input|KeyboardEvents|E
  (params (Key :type Key%20Structure :default "None"))
  (bind _isactive (Variables|Default|GetIsActive))
  (:Pressed
    (if _isactive
      (Rendering|Components|TextRender|SetText (Variables|Default|GetFrontText) (Utilities|Text|ToText(String) ""))
      (if (Variables|Default|GetIsOpen)
        (Transformation|AddLocalOffset (Variables|Default|GetDoor) "0.000000,0.000000,-330.000000" false false)
        (Variables|Default|SetIsOpen false)
        (else
          (Transformation|AddLocalOffset (Variables|Default|GetDoor) "0.000000,0.000000,330.000000" false false)
          (Variables|Default|SetIsOpen true)))
      (elif (>= (Variables|/Game/FirstPerson/Blueprints/BP_FirstPersonCharacter.BP_FirstPersonCharacter_C|GetnumOfComponents (Variables|Default|GetCharacterReference)) 2)
        (bind _returnvalue (Utilities|Time|SetTimerbyEvent (delegate Custom|FixDoor) 1.2))
        (Variables|Default|SetTimer%20Reference _returnvalue)
        (Rendering|Components|TextRender|SetText (Variables|Default|GetFrontText) (Utilities|Text|ToText(String) "Fixing Door..."))
        (else
          (Rendering|Components|TextRender|SetText (Variables|Default|GetFrontText) (Utilities|Text|ToText(String) "Insufficient Components"))))))
  (:Released
    (if (not _isactive)
      (Utilities|Time|ClearandInvalidateTimerbyHandle (Variables|Default|GetTimer%20Reference))
      (Rendering|Components|TextRender|SetText (Variables|Default|GetFrontText) (Utilities|Text|ToText(String) "Press E to Fix the Door")))))

(fn ConstructionScript)