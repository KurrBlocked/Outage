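; BP_PowerBox is a one-time pickup that the first-person character collects by holding E inside its overlap box.
; Overlapping while active enables input and shows a text prompt; leaving disables input and clears the timer.
; Holding E runs a short cancelable timer that deactivates the box, calls CollectOrbs on the player and plays a sound.
; Tick applies the base material to the light mesh whenever the box is inactive.
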(event OnComponentBeginOverlap(Box)
  (params (OverlappedComponent :type Primitive%20Component%20Object%20Reference) (OtherActor :type Actor%20Object%20Reference) (OtherComp :type Primitive%20Component%20Object%20Reference) (OtherBodyIndex :type Integer) (bFromSweep :type Boolean) (SweepResult :type Hit%20Result%20Structure%20%28by%20ref%29))
  (bind _asbp_first_person_character (Utilities|Casting|CastToBP_FirstPersonCharacter OtherActor))
  (if (Variables|Default|GetIsActive)
    (Input|EnableInput (Game|GetPlayerController 0))
    (Rendering|Components|TextRender|SetText (Variables|Default|GetTextRender) (Utilities|Text|ToText(String) "Hold E to Collect"))
    (Variables|Default|SetPlayerReference _asbp_first_person_character)))

(event OnComponentEndOverlap(Box)
  (params (OverlappedComponent :type Primitive%20Component%20Object%20Reference) (OtherActor :type Actor%20Object%20Reference) (OtherComp :type Primitive%20Component%20Object%20Reference) (OtherBodyIndex :type Integer))
  (Utilities|Casting|CastToBP_FirstPersonCharacter OtherActor)
  (Input|DisableInput (Game|GetPlayerController 0))
  (Rendering|Components|TextRender|SetText (Variables|Default|GetTextRender) (Utilities|Text|ToText(String) ""))
  (Utilities|Time|ClearandInvalidateTimerbyHandle (Variables|Default|GetTimerReference)))

(event Custom|Collect
  (Variables|Default|SetIsActive false)
  (Rendering|Components|TextRender|SetText (Variables|Default|GetTextRender) (Utilities|Text|ToText(String) ""))
  (Default|CollectOrbs (Variables|Default|GetPlayerReference))
  (Audio|Components|Audio|Play (Variables|Default|GetSound) 0.0))

(event EventTick
  (params (DeltaSeconds :type Float%20%28single-precision%29))
  (if (not (Variables|Default|GetIsActive))
    (Rendering|Material|SetMaterial (Variables|Default|GetLight) 0 "/Game/FPWeapon/Materials/BaseMaterial.BaseMaterial")))

(event Input|KeyboardEvents|E
  (params (Key :type Key%20Structure :default "None"))
  (:Pressed
    (if (Variables|Default|GetIsActive)
      (bind _returnvalue (Utilities|Time|SetTimerbyEvent (delegate Custom|Collect) 0.8))
      (Variables|Default|SetTimerReference _returnvalue)
      (Rendering|Components|TextRender|SetText (Variables|Default|GetTextRender) (Utilities|Text|ToText(String) "Collecting..."))))
  (:Released
    (Utilities|Time|ClearandInvalidateTimerbyHandle (Variables|Default|GetTimerReference))
    (if (Variables|Default|GetIsActive)
      (Rendering|Components|TextRender|SetText (Variables|Default|GetTextRender) (Utilities|Text|ToText(String) "Hold E to Collect")))))

(fn ConstructionScript
  (Variables|Default|SetIsActive true))