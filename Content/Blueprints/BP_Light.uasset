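; BP_Light is a light actor that goes dark while a BP_BlueGhost is inside either of its two trigger boxes.
; Begin and end overlap events on Box and Box1 set one flag per box.
; Tick polls both flags every frame, setting the SpotLight intensity and swapping the Cube material between lit and base.
; The construction script sets IsLit, which the graphs shown never read.
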(event OnComponentBeginOverlap(Box)
  (params (OverlappedComponent :type Primitive%20Component%20Object%20Reference) (OtherActor :type Actor%20Object%20Reference) (OtherComp :type Primitive%20Component%20Object%20Reference) (OtherBodyIndex :type Integer) (bFromSweep :type Boolean) (SweepResult :type Hit%20Result%20Structure%20%28by%20ref%29))
  (Utilities|Casting|CastToBP_BlueGhost OtherActor)
  (Variables|Default|SetIsBox1Overlapped true))

(event OnComponentEndOverlap(Box)
  (params (OverlappedComponent :type Primitive%20Component%20Object%20Reference) (OtherActor :type Actor%20Object%20Reference) (OtherComp :type Primitive%20Component%20Object%20Reference) (OtherBodyIndex :type Integer))
  (Utilities|Casting|CastToBP_BlueGhost OtherActor)
  (Variables|Default|SetIsBox1Overlapped false))

(event OnComponentBeginOverlap(Box1)
  (params (OverlappedComponent :type Primitive%20Component%20Object%20Reference) (OtherActor :type Actor%20Object%20Reference) (OtherComp :type Primitive%20Component%20Object%20Reference) (OtherBodyIndex :type Integer) (bFromSweep :type Boolean) (SweepResult :type Hit%20Result%20Structure%20%28by%20ref%29))
  (Utilities|Casting|CastToBP_BlueGhost OtherActor)
  (Variables|Default|SetIsBox2Overlapped true))

(event OnComponentEndOverlap(Box1)
  (params (OverlappedComponent :type Primitive%20Component%20Object%20Reference) (OtherActor :type Actor%20Object%20Reference) (OtherComp :type Primitive%20Component%20Object%20Reference) (OtherBodyIndex :type Integer))
  (Utilities|Casting|CastToBP_BlueGhost OtherActor)
  (Variables|Default|SetIsBox2Overlapped false))

(event EventTick
  (params (DeltaSeconds :type Float%20%28single-precision%29))
  (if (or (Variables|Default|GetIsBox1Overlapped) (Variables|Default|GetIsBox2Overlapped))
    (Rendering|Components|Light|SetIntensity (Variables|Default|GetSpotLight) 0.0)
    (Rendering|Material|SetMaterial (Variables|Default|GetCube) 0 "/Game/FPWeapon/Materials/BaseMaterial.BaseMaterial")
    (else
      (Rendering|Components|Light|SetIntensity (Variables|Default|GetSpotLight) 4e+01)
      (Rendering|Material|SetMaterial (Variables|Default|GetCube) 0 "/Game/Materials/M_Light.M_Light"))))

(fn ConstructionScript
  (Variables|Default|SetIsLit true))