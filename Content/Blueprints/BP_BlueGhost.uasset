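; Blue ghost enemy, a flipbook billboard that loads LoseScreen on touching the player, unless the player is exploding, which triggers its delayed teleport respawn.
; It wanders the navmesh, screams when Pawn Sensing spots someone, then chases for a limited time.
; Holding three orbs makes it pursue the player from Tick.
; A closed door touching it starts a timer that bleeds the door blue, then makes it temporarily phasable.
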(event OnSeePawn(PawnSensing)
  (params (Pawn :type Pawn%20Object%20Reference))
  (bind _self self)
  (bind _audio (Variables|Default|GetAudio))
  (if (Variables|Default|GetIsChasing)
    (CallFunction|StartChase)
    (elif (<= (Class|KismetSystemLibrary|GetTimerElapsedTimeHandle (Variables|Default|GetChaseWaitTimer)) 0.0)
      (bind _returnvalue (Utilities|Time|SetTimerbyEvent (delegate Custom|StartChase) 2.0))
      (Variables|Default|SetChaseWaitTimer _returnvalue)
      (Sprite|SetFlipbook (Variables|Default|GetPaperFlipbook) "/Game/Sprites/GhostScream/GhostScream.GhostScream")
      (AI|AIMoveTo _self (Transformation|GetActorLocation _self) 0 5.0 false
        (:then
          (Audio|Components|Audio|SetSound _audio "/Game/Audio/GhostScream.GhostScream")
          (Audio|Components|Audio|Play _audio 0.0)
          (Audio|Components|Audio|SetSound (Variables|Default|GetConstantAudio) 0))))))

(event OnComponentBeginOverlap(PlayerAttackRange)
  (params (OverlappedComponent :type Primitive%20Component%20Object%20Reference) (OtherActor :type Actor%20Object%20Reference) (OtherComp :type Primitive%20Component%20Object%20Reference) (OtherBodyIndex :type Integer) (bFromSweep :type Boolean) (SweepResult :type Hit%20Result%20Structure%20%28by%20ref%29))
  (bind _asbp_first_person_character (Utilities|Casting|CastToBP_FirstPersonCharacter OtherActor))
  (if (Variables|/Game/FirstPerson/Blueprints/BP_FirstPersonCharacter.BP_FirstPersonCharacter_C|GetIsExploding _asbp_first_person_character)
    (if (Variables|Default|GetCanKill)
      (CallFunction|Respawn))
    (elif (Variables|Default|GetCanKill)
      (Game|OpenLevel(byName) "LoseScreen"))))

(event OnComponentBeginOverlap(DoorChecker)
  (params (OverlappedComponent :type Primitive%20Component%20Object%20Reference) (OtherActor :type Actor%20Object%20Reference) (OtherComp :type Primitive%20Component%20Object%20Reference) (OtherBodyIndex :type Integer) (bFromSweep :type Boolean) (SweepResult :type Hit%20Result%20Structure%20%28by%20ref%29))
  (bind _asbp_door (Utilities|Casting|CastToBP_Door OtherActor))
  (bind _output_get (Variables|Default|SetCurrentDoor _asbp_door)))

(event OnComponentEndOverlap(DoorChecker)
  (params (OverlappedComponent :type Primitive%20Component%20Object%20Reference) (OtherActor :type Actor%20Object%20Reference) (OtherComp :type Primitive%20Component%20Object%20Reference) (OtherBodyIndex :type Integer))
  (bind _asbp_door (Utilities|Casting|CastToBP_Door OtherActor))
  (Utilities|Time|ClearandInvalidateTimerbyHandle (Variables|Default|GetTimerReference))
  (Variables|Default|SetIsPhasing false)
  (Variables|/Game/Blueprints/BP_Door.BP_Door_C|SetIsBleedingBlue _asbp_door false))

(event Custom|StartChase
  (bind _constantaudio (Variables|Default|GetConstantAudio))
  (bind _constantaudio_2 (Variables|Default|GetConstantAudio))
  (Variables|Default|SetIsChasing true)
  (Utilities|FlowControl|Sequence
    (:then_0
      (Variables|/Script/Engine.CharacterMovementComponent|SetMaxWalkSpeed (Variables|Character|GetCharacterMovement) 4.8e+02)
      (Sprite|SetFlipbook (Variables|Default|GetPaperFlipbook) "/Game/Sprites/GhostChase/GhostChase.GhostChase")
      (Audio|Components|Audio|SetSound _constantaudio "/Game/Audio/GhostPatrol.GhostPatrol")
      (Audio|Components|Audio|Play _constantaudio 0.0))
    (:then_1
      (AI|AIMoveTo self "0, 0, 0" (stale OnSeePawn(PawnSensing) Pawn) 5.0 false
        (:then
          (Utilities|FlowControl|RetriggerableDelay 7.0)
          (Variables|/Script/Engine.CharacterMovementComponent|SetMaxWalkSpeed (Variables|Character|GetCharacterMovement) 2.5e+02)
          (CallFunction|MovetoRandomLocation)
          (Sprite|SetFlipbook (Variables|Default|GetPaperFlipbook) "/Game/Sprites/GhostPatrol/GhostPatrol.GhostPatrol")
          (Variables|Default|SetIsChasing false)
          (Audio|Components|Audio|SetSound _constantaudio_2 "/Game/Audio/GhostPatrol.GhostPatrol")
          (Audio|Components|Audio|Play _constantaudio_2 0.0))))))

(event Custom|MoveToRandomLocation
  (bind _randomlocation (Class|NavigationSystemV1|GetRandomLocationinNavigableRadius (Transformation|GetActorLocation) 3e+03 0 0))
  (AI|AIMoveTo self _randomlocation 0 5.0 false
    (:OnSuccess
      (Utilities|Time|SetTimerbyEvent (delegate Custom|MoveAgain) 2.0))))

(event Custom|PhaseFromDoorChange
  (Default|MakeDoorTemporarilyPhasable (Variables|Default|GetCurrentDoor)))

(event Custom|Respawn
  (bind _audio (Variables|Default|GetAudio))
  (Utilities|Time|SetTimerbyEvent (delegate Custom|Reset) 1.5)
  (Audio|Components|Audio|SetSound _audio "/Game/Audio/GhostDeath.GhostDeath")
  (Audio|Components|Audio|Play _audio 0.0)
  (Variables|/Script/Engine.CharacterMovementComponent|SetMaxWalkSpeed (Variables|Character|GetCharacterMovement) 0.1)
  (Variables|Default|SetCanKill false))

(event Custom|PhaseThroughDoor
  (Default|MakeDoorTemporarilyPhasable (stale OnComponentBeginOverlap(DoorChecker) _output_get)))

(event Custom|Reset
  (bind _playerreference (Variables|Default|GetPlayerReference))
  (bind _capsulecomponent (Variables|/Script/Engine.Character|GetCapsuleComponent _playerreference))
  (bind _returnvalue (Transformation|GetWorldLocation _capsulecomponent))
  (Variables|/Script/Engine.CharacterMovementComponent|SetMaxWalkSpeed (Variables|Character|GetCharacterMovement) 4.8e+02)
  (Variables|Default|SetIsChasing false)
  (bind _randomlocation (Class|NavigationSystemV1|GetRandomLocationinNavigableRadius _returnvalue 1e+04 0 0))
  (if (< (Math|Vector|Distance(Vector) _randomlocation _returnvalue) 1e+03)
    (Class|NavigationSystemV1|GetRandomLocationinNavigableRadius _returnvalue 1e+04 0 0)
    (Transformation|Teleport "0, 0, 0" "0, 0, 0")
    (Variables|Default|SetCanKill true)
    (else
      (Transformation|Teleport _randomlocation "0, 0, 0")
      (Variables|Default|SetCanKill true))))

(event Custom|MoveAgain
  (CallFunction|MovetoRandomLocation))

(event EventTick
  (params (DeltaSeconds :type Float%20%28single-precision%29))
  (bind _currentdoor (Variables|Default|GetCurrentDoor))
  (bind _paperflipbook (Variables|Default|GetPaperFlipbook))
  (Utilities|FlowControl|Sequence
    (:then_0
      (if (Utilities|IsValid _currentdoor)
        (if (Math|Boolean|ANDBoolean (not (Variables|/Game/Blueprints/BP_Door.BP_Door_C|GetIsOpen _currentdoor)) (Variables|/Game/Blueprints/BP_Door.BP_Door_C|GetIsDoorTouchingGhost _currentdoor) (not (Variables|Default|GetIsPhasing)))
          (bind _returnvalue (Utilities|Time|SetTimerbyEvent (delegate Custom|PhaseFromDoorChange) 3.0))
          (Variables|Default|SetTimerReference _returnvalue)
          (Variables|Default|SetIsPhasing true)
          (Variables|/Game/Blueprints/BP_Door.BP_Door_C|SetIsBleedingBlue _currentdoor true))))
    (:then_1
      (if (Variables|Default|GetIsPhasing)
        (Transformation|SetWorldRotation _paperflipbook (Transformation|GetActorRotation _currentdoor) false false)
        (else
          (Transformation|SetWorldRotation _paperflipbook (Math|Conversions|RotationFromXVector (.Y (Math|Rotator|GetAxes (Math|Rotator|FindLookatRotation (Transformation|GetActorLocation) (Transformation|GetActorLocation (Game|GetPlayerCameraManager 0)))))) false false))))
    (:then_2
      (if (and (== (Variables|/Game/FirstPerson/Blueprints/BP_FirstPersonCharacter.BP_FirstPersonCharacter_C|GetnumOfOrbs (Variables|Default|GetPlayerReference)) 3) (not (Variables|Default|GetIsChasing)))
        (AI|AIMoveTo self "0, 0, 0" (Variables|Default|GetPlayerReference) 5.0 false
          (:then
            (Variables|/Script/Engine.CharacterMovementComponent|SetMaxWalkSpeed (Variables|Character|GetCharacterMovement) 4.8e+02)))))))

(event EventBeginPlay
  (CallFunction|MovetoRandomLocation)
  (bind _returnvalue (Actor|GetActorOfClass "/Game/FirstPerson/Blueprints/BP_FirstPersonCharacter.BP_FirstPersonCharacter_C"))
  (Variables|Default|SetPlayerReference _returnvalue)
  (Variables|Default|SetCanKill true))

(fn ConstructionScript)