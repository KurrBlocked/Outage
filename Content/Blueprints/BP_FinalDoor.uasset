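; BP_FinalDoor is the level's exit: a console that needs three orbs to power, and a door that loads the WinScreen level once powered.
; Overlaps with the console and door collisions toggle input and prompt text for the first-person character.
; Pressing E at the console sets IsActive when the player holds three orbs, and pressing E at the active door wins.
; While active, Tick reapplies the lit material to three door lights every frame.
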(event OnComponentBeginOverlap(ConsoleCollision)
  (params (OverlappedComponent :type Primitive%20Component%20Object%20Reference) (OtherActor :type Actor%20Object%20Reference) (OtherComp :type Primitive%20Component%20Object%20Reference) (OtherBodyIndex :type Integer) (bFromSweep :type Boolean) (SweepResult :type Hit%20Result%20Structure%20%28by%20ref%29))
  (bind _asbp_first_person_character (Utilities|Casting|CastToBP_FirstPersonCharacter OtherActor))
  (Variables|Default|SetPlayerReference _asbp_first_person_character)
  (Input|EnableInput (Game|GetPlayerController 0))
  (if (== (Variables|/Game/FirstPerson/Blueprints/BP_FirstPersonCharacter.BP_FirstPersonCharacter_C|GetnumOfOrbs (Variables|Default|GetPlayerReference)) 3)
    (Rendering|Components|TextRender|SetText (Variables|Default|GetConsoleText) (Utilities|Text|ToText(String) "Press E to Power the Console"))
    (else
      (Rendering|Components|TextRender|SetText (Variables|Default|GetConsoleText) (Utilities|Text|ToText(String) "Requires 3 Orbs to Power"))))
  (Variables|Default|SetIsTouching%20Console true))

(event OnComponentEndOverlap(ConsoleCollision)
  (params (OverlappedComponent :type Primitive%20Component%20Object%20Reference) (OtherActor :type Actor%20Object%20Reference) (OtherComp :type Primitive%20Component%20Object%20Reference) (OtherBodyIndex :type Integer))
  (Utilities|Casting|CastToBP_FirstPersonCharacter OtherActor)
  (Input|DisableInput (Game|GetPlayerController 0))
  (Rendering|Components|TextRender|SetText (Variables|Default|GetConsoleText) (Utilities|Text|ToText(String) ""))
  (Variables|Default|SetIsTouching%20Console false))

(event OnComponentBeginOverlap(DoorCollision)
  (params (OverlappedComponent :type Primitive%20Component%20Object%20Reference) (OtherActor :type Actor%20Object%20Reference) (OtherComp :type Primitive%20Component%20Object%20Reference) (OtherBodyIndex :type Integer) (bFromSweep :type Boolean) (SweepResult :type Hit%20Result%20Structure%20%28by%20ref%29))
  (Utilities|Casting|CastToBP_FirstPersonCharacter OtherActor)
  (if (Variables|Default|GetIsActive)
    (Input|EnableInput (Game|GetPlayerController 0))
    (Rendering|Components|TextRender|SetText (Variables|Default|GetDoorText) (Utilities|Text|ToText(String) "Press E To Open Door"))
    (Variables|Default|SetIsTouchingDoor true)))

(event OnComponentEndOverlap(DoorCollision)
  (params (OverlappedComponent :type Primitive%20Component%20Object%20Reference) (OtherActor :type Actor%20Object%20Reference) (OtherComp :type Primitive%20Component%20Object%20Reference) (OtherBodyIndex :type Integer))
  (Utilities|Casting|CastToBP_FirstPersonCharacter OtherActor)
  (Input|DisableInput (Game|GetPlayerController 0))
  (Rendering|Components|TextRender|SetText (Variables|Default|GetDoorText) (Utilities|Text|ToText(String) ""))
  (Variables|Default|SetIsTouchingDoor false))

(event EventTick
  (params (DeltaSeconds :type Float%20%28single-precision%29))
  (if (Variables|Default|GetIsActive)
    (Rendering|Material|SetMaterial (Variables|Default|GetDoorLight) 0 "/Game/Materials/M_Light.M_Light")))

(event Input|KeyboardEvents|E
  (params (Key :type Key%20Structure :default "None"))
  (:Pressed
    (if (and (Variables|Default|GetIsTouching%20Console) (not (Variables|Default|GetIsActive)))
      (if (== (Variables|/Game/FirstPerson/Blueprints/BP_FirstPersonCharacter.BP_FirstPersonCharacter_C|GetnumOfOrbs (Variables|Default|GetPlayerReference)) 3)
        (Variables|Default|SetIsActive true)
        (Rendering|Components|TextRender|SetText (Variables|Default|GetConsoleText) (Utilities|Text|ToText(String) "")))
      (elif (and (Variables|Default|GetIsTouchingDoor) (Variables|Default|GetIsActive))
        (Game|OpenLevel(byName) "WinScreen")))))

(fn ConstructionScript)